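; BP_MyPlayer is the player character Blueprint, providing events to start and stop swimming.
; StartSwimming gives a slight launch along the actor's up vector, flags the movement component's current physics volume as water and sets IsSwimming.
; StopSwimming clears both flags.
; The water state is toggled on the physics volume itself rather than by setting the movement mode, and nothing in this graph calls either event.
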(event `self.ReceiveBeginPlay`)

(event `StartSwimming`
  ;[1 1 1] Is Swimming
  ;;[1 1 1] StartSwimming
  (`self.LaunchCharacter` (* (`KismetMathLibrary.GetUpVector` (`self.K2_GetActorRotation`)) 2.0))
  (set `PhysicsVolume.bWaterVolume` true (`MovementComponent.GetPhysicsVolume` (`self.CharacterMovement`)))
  (set `self.isSwimming` true))

(event `StopSwimming`
  ;[1 1 1] Is Swimming
  ;;[1 1 1] StopSwimming
  (set `PhysicsVolume.bWaterVolume` false (`MovementComponent.GetPhysicsVolume` (`self.CharacterMovement`)))
  (set `self.isSwimming` false))

(fn `UserConstructionScript`)